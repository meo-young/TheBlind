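; Modular staircase building Blueprint for the house kit, assembled entirely in the construction script, with no active runtime logic.
; The Stairs selection (basement, main or straight, left or right) and the ExtraRailing flag pick which child actor component to add and cache its children.
; Floor and Ceiling toggles raise the matching side's opening pieces one storey or destroy them; unused sides, and both for basement stairs, are destroyed.
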(event EventBeginPlay)

(event Collision|EventActorBeginOverlap
  (params (OtherActor :type Actor%20Object%20Reference)))

(event EventTick
  (params (DeltaSeconds :type Float%20%28single-precision%29)))

(fn ConstructionScript
  (bind _floor_6x3_stairs_l (Variables|Default|GetFloor_6x3_stairs_L))
  (bind _ceiling_6x3_stairs_l (Variables|Default|GetCeiling_6x3_stairs_L))
  (bind _floor_6x3_stairs_l_2 (Variables|Default|GetFloor_6x3_stairs_L))
  (bind _ceiling_6x3_stairs_l_2 (Variables|Default|GetCeiling_6x3_stairs_L))
  (bind _floor_6x3_stairs_r (Variables|Default|GetFloor_6x3_stairs_R))
  (bind _ceiling_6x3_stairs_r (Variables|Default|GetCeiling_6x3_stairs_R))
  (bind _floor_6x3_stairs_r_2 (Variables|Default|GetFloor_6x3_stairs_R))
  (bind _ceiling_6x3_stairs_r_2 (Variables|Default|GetCeiling_6x3_stairs_R))
  (if (Variables|Mesh|GetExtra%20Railing?)
    (switch Utilities|FlowControl|Switch|SwitchonE_Stairs (Variables|Mesh|GetStairs)
      (:NewEnumerator19
        (bind _returnvalue (AddComponent|AddChildActorComponent false))
        (bind _output_get (LocalVariables|SetChild%20Actor _returnvalue))
        (Variables|Mesh|SetStairs%20Components (Components|GetChildrenComponents _output_get true))
        (Components|DestroyComponent (Variables|Default|GetFloor_6x3_stairs_L) :!label _label)
        (Components|DestroyComponent (Variables|Default|GetCeiling_6x3_stairs_L))
        (Components|DestroyComponent (Variables|Default|GetFloor_6x3_stairs_R) :!label _label_2)
        (Components|DestroyComponent (Variables|Default|GetCeiling_6x3_stairs_R)))
      (:NewEnumerator25
        (bind _returnvalue_2 (AddComponent|AddChildActorComponent false))
        (bind _output_get_2 (LocalVariables|SetChild%20Actor _returnvalue_2))
        (Variables|Mesh|SetStairs%20Components (Components|GetChildrenComponents _output_get_2 true))
        (if (Variables|Mesh|GetFloor?) :!label _label_3
          (Transformation|SetRelativeLocationAndRotation _floor_6x3_stairs_l "0,0.000000,300.000000" "0, 0, 0" false false)
          (else
            (Components|DestroyComponent _floor_6x3_stairs_l)))
        (if (Variables|Mesh|GetCeiling?)
          (Transformation|SetRelativeLocationAndRotation _ceiling_6x3_stairs_l "0,0.000000,300.000000" "0, 0, 0" false false)
          (goto _label_2)
          (else
            (Components|DestroyComponent _ceiling_6x3_stairs_l)
            (goto _label_2))))
      (:NewEnumerator54
        (bind _returnvalue_3 (AddComponent|AddChildActorComponent false))
        (bind _output_get_3 (LocalVariables|SetChild%20Actor _returnvalue_3))
        (Variables|Mesh|SetStairs%20Components (Components|GetChildrenComponents _output_get_3 true))
        (if (Variables|Mesh|GetFloor?) :!label _label_4
          (Transformation|SetRelativeLocationAndRotation _floor_6x3_stairs_r "0, 0,300.000000" "0, 0, 0" false false)
          (else
            (Components|DestroyComponent _floor_6x3_stairs_r)))
        (if (Variables|Mesh|GetCeiling?)
          (Transformation|SetRelativeLocationAndRotation _ceiling_6x3_stairs_r "0, 0,300.000000" "0, 0, 0" false false)
          (else
            (Components|DestroyComponent _ceiling_6x3_stairs_r)))
        (Components|DestroyComponent (Variables|Default|GetFloor_6x3_stairs_L))
        (Components|DestroyComponent (Variables|Default|GetCeiling_6x3_stairs_L)))
      (:NewEnumerator55
        (bind _returnvalue_4 (AddComponent|AddChildActorComponent false))
        (bind _output_get_4 (LocalVariables|SetChild%20Actor _returnvalue_4))
        (Variables|Mesh|SetStairs%20Components (Components|GetChildrenComponents _output_get_4 true))
        (goto _label_3))
      (:NewEnumerator56
        (bind _returnvalue_5 (AddComponent|AddChildActorComponent false))
        (bind _output_get_5 (LocalVariables|SetChild%20Actor _returnvalue_5))
        (Variables|Mesh|SetStairs%20Components (Components|GetChildrenComponents _output_get_5 true))
        (goto _label_4)))
    (else
      (switch Utilities|FlowControl|Switch|SwitchonE_Stairs (Variables|Mesh|GetStairs)
        (:NewEnumerator19
          (bind _returnvalue_6 (AddComponent|AddChildActorComponent false))
          (bind _output_get_6 (LocalVariables|SetChild%20Actor _returnvalue_6))
          (Variables|Mesh|SetStairs%20Components (Components|GetChildrenComponents _output_get_6 true))
          (goto _label))
        (:NewEnumerator25
          (bind _returnvalue_7 (AddComponent|AddChildActorComponent false))
          (bind _output_get_7 (LocalVariables|SetChild%20Actor _returnvalue_7))
          (Variables|Mesh|SetStairs%20Components (Components|GetChildrenComponents _output_get_7 true))
          (if (Variables|Mesh|GetFloor?) :!label _label_5
            (Transformation|SetRelativeLocationAndRotation _floor_6x3_stairs_l_2 "0,0.000000,300.000000" "0, 0, 0" false false)
            (else
              (Components|DestroyComponent _floor_6x3_stairs_l_2)))
          (if (Variables|Mesh|GetCeiling?)
            (Transformation|SetRelativeLocationAndRotation _ceiling_6x3_stairs_l_2 "0,0.000000,300.000000" "0, 0, 0" false false)
            (else
              (Components|DestroyComponent _ceiling_6x3_stairs_l_2)))
          (Components|DestroyComponent (Variables|Default|GetFloor_6x3_stairs_R))
          (Components|DestroyComponent (Variables|Default|GetCeiling_6x3_stairs_R)))
        (:NewEnumerator54
          (bind _returnvalue_8 (AddComponent|AddChildActorComponent false))
          (bind _output_get_8 (LocalVariables|SetChild%20Actor _returnvalue_8))
          (Variables|Mesh|SetStairs%20Components (Components|GetChildrenComponents _output_get_8 true))
          (if (Variables|Mesh|GetFloor?) :!label _label_6
            (Transformation|SetRelativeLocationAndRotation _floor_6x3_stairs_r_2 "0, 0,300.000000" "0, 0, 0" false false)
            (else
              (Components|DestroyComponent _floor_6x3_stairs_r_2)))
          (if (Variables|Mesh|GetCeiling?)
            (Transformation|SetRelativeLocationAndRotation _ceiling_6x3_stairs_r_2 "0, 0,300.000000" "0, 0, 0" false false)
            (else
              (Components|DestroyComponent _ceiling_6x3_stairs_r_2)))
          (Components|DestroyComponent (Variables|Default|GetFloor_6x3_stairs_L))
          (Components|DestroyComponent (Variables|Default|GetCeiling_6x3_stairs_L)))
        (:NewEnumerator55
          (bind _returnvalue_9 (AddComponent|AddChildActorComponent false))
          (bind _output_get_9 (LocalVariables|SetChild%20Actor _returnvalue_9))
          (Variables|Mesh|SetStairs%20Components (Components|GetChildrenComponents _output_get_9 true))
          (goto _label_5))
        (:NewEnumerator56
          (bind _returnvalue_10 (AddComponent|AddChildActorComponent false))
          (bind _output_get_10 (LocalVariables|SetChild%20Actor _returnvalue_10))
          (Variables|Mesh|SetStairs%20Components (Components|GetChildrenComponents _output_get_10 true))
          (goto _label_6))))))