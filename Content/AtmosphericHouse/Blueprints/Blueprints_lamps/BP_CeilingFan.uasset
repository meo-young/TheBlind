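; BP_CeilingFan is a ceiling fan prop with a built-in lamp that can be set lit or unlit.
; The construction script uses LampOn to apply lit or off materials to the base, blades and lamp meshes, destroying the point light when off.
; On BeginPlay, a timeline rotates the blades regardless of lamp state, adding its track value as relative yaw each update, so the increments are not scaled by delta time.
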(event EventBeginPlay
  (bind _newtrack_0 (Timeline|Timeline_0 Play)
    (:Update
      (Transformation|AddRelativeRotation (Variables|Default|GetCeilingFan_Blades) (Math|Rotator|MakeRotator 0.0 0.0 _newtrack_0) false false))))

(fn ConstructionScript
  (if (Variables|Lamp|GetLamp%20On?)
    (Rendering|Material|SetMaterial (Variables|Default|GetCeilingFan_Base) 0 "/Game/AtmosphericHouse/Materials/Clean/MI_CeilingFan_clean.MI_CeilingFan_clean")
    (Rendering|Material|SetMaterial (Variables|Default|GetCeilingFan_Blades) 0 "/Game/AtmosphericHouse/Materials/Clean/MI_CeilingFan_clean.MI_CeilingFan_clean")
    (Rendering|Material|SetMaterial (Variables|Default|GetCeilingFan_Lamps) 0 "/Game/AtmosphericHouse/Materials/Clean/MI_CeilingFan_clean.MI_CeilingFan_clean")
    (else
      (Components|DestroyComponent (Variables|Default|GetPointLight))
      (Rendering|Material|SetMaterial (Variables|Default|GetCeilingFan_Base) 0 "/Game/AtmosphericHouse/Materials/Clean/MI_CeilingFan_off_clean.MI_CeilingFan_off_clean")
      (Rendering|Material|SetMaterial (Variables|Default|GetCeilingFan_Blades) 0 "/Game/AtmosphericHouse/Materials/Clean/MI_CeilingFan_off_clean.MI_CeilingFan_off_clean")
      (Rendering|Material|SetMaterial (Variables|Default|GetCeilingFan_Lamps) 0 "/Game/AtmosphericHouse/Materials/Clean/MI_CeilingFan_off_clean.MI_CeilingFan_off_clean"))))