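; BP_Doll is a doll enemy Blueprint with a skinned Body and a runtime-assembled Cloth mesh.
; On BeginPlay it merges skeletal meshes from its merge parameters, assigns the result to Cloth and sets Body as its leader pose component.
; Every tick it drives the Body's Scream and AngryPain morph targets from a single ScreamValue, which this graph only reads.
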(event EventBeginPlay
  (bind _cloth (Variables|Default|GetCloth))
  (bind _returnvalue (Class|SkeletalMergingLibrary|MergeMeshes (Variables|Default|GetSkeletalMeshMergingParams)))
  (Components|SkeletalMesh|SetSkeletalMeshAsset _cloth _returnvalue)
  (Components|SkinnedMesh|SetLeaderPoseComponent _cloth (Variables|Default|GetBody) false false))

(event EventTick
  (params (DeltaSeconds :type Float%20%28single-precision%29))
  (Components|SkeletalMesh|SetMorphTarget (Variables|Default|GetBody) "Scream" (Variables|Default|GetScreamValue) true)
  (Components|SkeletalMesh|SetMorphTarget (Variables|Default|GetBody) "AngryPain" (Variables|Default|GetScreamValue) true))

(fn ConstructionScript)